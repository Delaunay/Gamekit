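; Prototype base Gameplay Ability that branches on the static data's behavior: Hidden commits instantly, Actor/Point Target call native activation, and others are unimplemented.
; The point-target event spawns or reuses a configured targeting actor, awaits confirmed target data, then moves the avatar within cast range.
; It then plays a montage whose cast-point event triggers a server-only commit, projectile spawn and ability end, with debug prints throughout.
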(event `self.K2_ActivateAbility`
  (bind (_abilitystatic _valid) (`self.K2_GetAbilityStatic`))
  (if _valid
    (set `self.Ability Behavior` (`.AbilityBehavior` (break `GKAbilityStatic` _abilitystatic)))
    (else
      (set `self.Ability Behavior` "Hidden")))
  (switch `EGK_AbilityBehavior` (`self.Ability Behavior`)
    (:`Hidden`
      (`KismetSystemLibrary.PrintString` "Commit")
      (bind _returnvalue (`self.K2_CommitAbility`))
      (if _returnvalue
        (`self.K2_EndAbility`)
        (`KismetSystemLibrary.PrintString` (`KismetStringLibrary.Concat_StrStr` "Ability at: "))
        (else
          (`self.K2_CancelAbility`))))
    (:`Passive`
      (`KismetSystemLibrary.PrintString` "Not Implemented" :!label _label))
    (:`NoTarget`
      (goto _label))
    (:`ActorTarget`
      (`self.ActivateAbility_Native` :!label _label_2))
    (:`PointTarget`
      (goto _label_2))
    (:`Toggle`
      (goto _label))))

(event `ActivateAbility_PointTarget`
  (bind (_returnvalue_owneractor _returnvalue_avataractor) (break `GameplayAbilityActorInfo` (`self.GetActorInfo`)))
  (bind _aspawn (cast `Pawn` _returnvalue_avataractor))
  (set `self.Pawn` _aspawn)
  (`|ExecutionSequence`
    (:`then_0`
      (bind _abilitystatic (`self.K2_GetAbilityStatic`))
      (`KismetSystemLibrary.PrintString` (`KismetStringLibrary.Conv_NameToString` (break `GKAbilityStatic` _abilitystatic))))
    (:`then_1`
      (bind _abilitystatic_2 (`self.K2_GetAbilityStatic`))
      (`self.Spawn Ability Target Actor` _abilitystatic_2))
    (:`then_2`
      (bind (_asynctaskproxy _data) (`GKAbilityTask_WaitForTargetData.WaitForTargetDataUsingActor` "None" "UserConfirmed" (`self.TargetActor`))
        (:`ValidData`
          (bind _impactpoint (`self.Get Impact Point` _data))
          (`GKAbilityTask_MoveToDestination.MoveToDestination` "None" _impactpoint (`.CastMaxRange` (break `GKAbilityStatic` _abilitystatic)) 12.0 150.0
            (:`OnCompleted`
              (`KismetSystemLibrary.PrintString` "Move Completed")
              (bind (_asynctaskproxy_2 _eventtag _eventdata) (`GKAbilityTask_PlayMontageAndWaitForEvent.PlayMontageAndWaitForEvent` "None" "/Gamekit/Characters/Animations/Boxing_Montage.Boxing_Montage" (struct :`GameplayTags` (struct :`(TagName` "Animation.CastPoint"))) _data 2.0 "None" false)
                (:`then`
                  ;[1 1 1] Makes sure ability is always ended
                  (set `self.MontageTask` _asynctaskproxy_2))
                (:`OnCompleted`
                  (`KismetSystemLibrary.PrintString` "Completed")
                  (`self.K2_EndAbility`))
                (:`OnBlendOut`
                  (`KismetSystemLibrary.PrintString` "BlendOut")
                  (`self.K2_EndAbility`))
                (:`OnInterrupted`
                  (`KismetSystemLibrary.PrintString` "Interrupted")
                  (`self.K2_CancelAbility` :!label _label_3))
                (:`OnCancelled`
                  (`KismetSystemLibrary.PrintString` "Cancelled")
                  (goto _label_3))
                (:`EventReceived`
                  ;[1 1 1] Avoid double activation.
                  ; Only Server Commit
                  (`self.K2_HasAuthority`
                    (:`True`
                      (`KismetSystemLibrary.PrintString` "Commit")
                      (bind _returnvalue (`self.K2_CommitAbility`))
                      (if _returnvalue
                        (`|ExecutionSequence`
                          (:`then_0`
                            (`self.SpawnProjectile` _eventtag _eventdata)
                            (`self.SpawnProjectile_Done`))
                          (:`then_1`
                            (`self.K2_EndAbility` :!label _label_4))
                          (:`then_2`
                            (`KismetSystemLibrary.PrintString` (`KismetStringLibrary.Concat_StrStr` "Ability at: " (`KismetStringLibrary.Conv_VectorToString` _impactpoint)))
                            (`KismetSystemLibrary.DrawDebugCircle` _impactpoint 10.0 72 (struct :`R` 1.0 :`A` 1.0) 5.0 2.0 (0.0 1.0 0.0) (1.0 0.0 0.0) true)))
                        (else
                          (`self.K2_CancelAbility`))))))))))
        (:`Cancelled`
          (`self.K2_CancelAbility`)
          (`KismetSystemLibrary.PrintString` "Target Got cancelled"))))))

(event `EndAbilityAfterServer`
  ;[1 1 1] We have to introduce a delay here, to avoid the server from
  ; cancelling an ability that is being activated.
  ;
  ; Client Activate -> Select Target -> Replicates to Server -> End Ability
  ; Server Cancel Activation because Ability Ended and Target was not selected
  ;
  ; We slow the EndAbility by 0.12 which is half the standard human reaction time and abour 3.75 frames (30 fps)
  ;
  ; NB: We need to sync client & server right after the target data is ready OR we remove the WaitTarget Data async task to avoid too much traffic
  ;
  ; This is a hack, Note maybe we do not need this since blendout should be called all the time
  ;
  ; NOTE: NOW ONLY THE SERVER COMMITS SO this became a non issue
  (goto _label_4))

(event `SpawnProjectile_Done`
  (`KismetSystemLibrary.PrintString` "Spawned"))

(fn `Get Impact Point`
  (params (InputPin :type "GameplayAbilityTargetDataHandle Structure (by ref)"))
  (returns (ImpactPoint :type "Vector Structure"))
  (bind (_returnvalue_bblockinghit _returnvalue_binitialoverlap _returnvalue_time _returnvalue_distance _returnvalue_location _returnvalue_impactpoint) (`GameplayStatics.BreakHitResult` (`AbilitySystemBlueprintLibrary.GetHitResultFromTargetData` InputPin)))
  (if (`AbilitySystemBlueprintLibrary.TargetDataHasHitResult` InputPin)
    (`KismetSystemLibrary.PrintString` "Impact Point")
    (return _returnvalue_impactpoint)
    (elif (`AbilitySystemBlueprintLibrary.TargetDataHasActor` InputPin)
      (`KismetSystemLibrary.PrintString` "Actor Location")
      (return (`Actor.K2_GetActorLocation` (`|GetArrayItem` (`AbilitySystemBlueprintLibrary.GetActorsFromTargetData` InputPin))))
      (else
        (`KismetSystemLibrary.PrintString` "No Data")
        (return (0.0 0.0 0.0))))))

(fn `Spawn Ability Target Actor`
  (params (AbilityData :type "GKAbilityStatic Structure (by ref)"))
  (locals (`Trace Mode` :type Byte :default 0))
  (`/Engine/EditorBlueprintResources/StandardMacros.IsValid` (`self.TargetActor`)
    (:`Is Valid`
      (`KismetSystemLibrary.PrintString` "Reusing Target Actor"))
    (:`Is Not Valid`
      (bind _returnvalue (`|SpawnActorFromClass` :`Class` "/Gamekit/Abilities/Target/AControllerTrace_Traget.AControllerTrace_Traget_C" :`SpawnTransform` (`KismetMathLibrary.MakeTransform` (0.0 0.0 0.0)) :`CollisionHandlingOverride` "Undefined" :`TransformScaleMethod` "OverrideRootScale" :`ObjectTypes` AbilityData_TargetObjectTypes :`TargetMode` AbilityData_AbilityBehavior :`MaxRange` AbilityData_CastMaxRange :`MinRange` AbilityData_CastMinRange :`AreaOfEffect` AbilityData_AreaOfEffect :`ClassFilter` null :`TargetActorFaction` AbilityData_TargetActorFaction :`ReticleClass` null :`Instigator` null))
      (set `self.TargetActor` _returnvalue)
      (`KismetSystemLibrary.PrintString` "Spawning new targeting actor"))))